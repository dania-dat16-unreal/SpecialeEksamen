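; BuildingMaster is a building Blueprint for an RTS game, with a configurable display mesh and health-based damage handling.
; The construction script applies DisplayMesh to the static mesh component.
; AnyDamage sets CurrentHealth to damage minus current health, reversing the usual subtraction.
; When the result is at or below MaxHealth, it removes itself from a valid controller's MyBuildings and sets AutoDestroyWhenFinished rather than calling DestroyActor.
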(event `self.ReceiveTick`
  (params (DeltaSeconds :type "Float (single-precision)")))

(event `self.ReceiveAnyDamage`
  (params (Damage :type "Float (single-precision)") (DamageType :type "DamageType Object Reference") (InstigatedBy :type "Controller Object Reference") (DamageCauser :type "Actor Object Reference"))
  (bind _controllerref (`self.ControllerRef`))
  (bind _output_get (set `self.CurrentHealth` (- Damage (`self.CurrentHealth`))))
  (if (<= _output_get (`self.MaxHealth`))
    (if (`KismetSystemLibrary.IsValid` _controllerref)
      (`KismetArrayLibrary.Array_RemoveItem` (`/Game/MyRTSGame/Blueprints/CameraPawnController.MyBuildings` _controllerref) self)
      (set `self.bAutoDestroyWhenFinished` true))))

(fn `UserConstructionScript`
  (`StaticMeshComponent.SetStaticMesh` (`self.StaticMesh`) (`self.DisplayMesh`)))