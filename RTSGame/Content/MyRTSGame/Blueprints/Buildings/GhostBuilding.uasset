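; Placement preview actor for RTS build mode, showing a ghost mesh of the chosen building and toggling the controller's BuildModeActive flag.
; While active, a gated Tick snaps it to the grid at the cursor position and swaps to an error material when overlapping actors.
; ConstructBuilding2 briefly spawns a Barrack or Factory to read its class, proxy and mesh.
; GetConstructionStruct packages that data with the ghost's transform.
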(event `OnSpawn`
  (params (BuildingClass :type "/Game/MyRTSGame/Blueprints/Buildings/BuildingMaster Class Reference") (ConstructionProxy :type "/Game/MyRTSGame/Blueprints/Construction/ConstructionProxy Class Reference") (DisplayMesh :type "StaticMesh Object Reference"))
  ;[1 1 1] On spawn ghost
  (if (not (`self.IsActive`))
    (set `self.BuildingClass` BuildingClass)
    (set `self.ConstructionProxy` ConstructionProxy)
    (set `self.DisplayMesh` DisplayMesh)
    (set `self.IsActive` true)
    (set `/Game/MyRTSGame/Blueprints/CameraPawnController.BuildModeActive` true (`self.ControllerRef`))
    (`StaticMeshComponent.SetStaticMesh` (`self.GhostBuilding_Mesh`) (`self.DisplayMesh`))
    (`self.OpenTickGate`)
    (`self.SetMaterial` (not (`self.IsOverlapping`)))))

(event `KillGhost`
  ;[1 1 1] Kill ghost
  (set `self.BuildingClass` null)
  (set `self.ConstructionProxy` null)
  (`self.CloseTickGate`)
  (set `self.DisplayMesh` null)
  (set `self.IsActive` false)
  (set `/Game/MyRTSGame/Blueprints/CameraPawnController.BuildModeActive` false (`self.ControllerRef`))
  (`StaticMeshComponent.SetStaticMesh` (`self.GhostBuilding_Mesh`) (`self.DisplayMesh`)))

(event `self.ReceiveTick`
  (params (DeltaSeconds :type "Float (single-precision)"))
  ;[1 1 1] Tick
  (`/Engine/EditorBlueprintResources/StandardMacros.Gate` true :!label _label
    (:`Exit`
      (`self.K2_SetActorLocation` self (`self.SetGridSnapVector`) false false)
      (if (`self.CheckOverlap`)
        (`self.SetMaterial` true)
        (else
          (`self.SetMaterial` false))))))

(event `OpenTickGate`
  ;[1 1 1] Tick
  (goto _label :!via `Open`))

(event `ConstructBuilding2`
  (params (Building :type String))
  (bind _controllerref (`self.ControllerRef`))
  ;[1 1 1] Comment
  (if (`KismetStringLibrary.EqualEqual_StrStr` Building "Barrack")
    (bind _returnvalue (`|SpawnActorFromClass` "/Game/MyRTSGame/Blueprints/Buildings/Barrack.Barrack_C" (`KismetMathLibrary.MakeTransform` (0.0 0.0 0.0) (struct) (1.0 1.0 1.0)) "AlwaysSpawn" "OverrideRootScale" null _controllerref 0 100.0))
    (`|ExecutionSequence`
      (:`then_0`
        (bind _asbuilding_master (castclass `/Game/MyRTSGame/Blueprints/Buildings/BuildingMaster` (`GameplayStatics.GetObjectClass` _returnvalue)))
        (`self.KillGhost`)
        (`self.OnSpawn` _asbuilding_master (`/Game/MyRTSGame/Blueprints/Buildings/BuildingMaster.ConstructionProxy` _returnvalue) (`/Game/MyRTSGame/Blueprints/Buildings/BuildingMaster.DisplayMesh` _returnvalue)))
      (:`then_1`
        (`self.K2_DestroyActor` _returnvalue)))
    (else
      (bind _returnvalue_2 (`|SpawnActorFromClass` "/Game/MyRTSGame/Blueprints/Buildings/Factory.Factory_C" (`KismetMathLibrary.MakeTransform` (0.0 0.0 0.0)) "AlwaysSpawn" "OverrideRootScale" null _controllerref 0 100.0))
      (`|ExecutionSequence`
        (:`then_0`
          (bind _asbuilding_master_2 (castclass `/Game/MyRTSGame/Blueprints/Buildings/BuildingMaster` (`GameplayStatics.GetObjectClass` _returnvalue_2)))
          (`self.KillGhost`)
          (`self.OnSpawn` _asbuilding_master_2 (`/Game/MyRTSGame/Blueprints/Buildings/BuildingMaster.ConstructionProxy` _returnvalue_2) (`/Game/MyRTSGame/Blueprints/Buildings/BuildingMaster.DisplayMesh` _returnvalue_2)))
        (:`then_1`
          (`self.K2_DestroyActor` _returnvalue_2))))))

(event `CloseTickGate`
  ;[1 1 1] Tick
  (goto _label :!via `Close`))

(event `SetMaterial`
  (params (IsError :type Boolean))
  (bind _ghostbuilding_mesh (`self.GhostBuilding_Mesh`))
  (bind _returnvalue (`MeshComponent.GetMaterials` _ghostbuilding_mesh))
  ;[1 1 1] Set material on building depending on overlap
  (if (not (== IsError (`self.IsOverlapping`)))
    (bind _output_get (set `self.IsOverlapping` IsError))
    (if _output_get
      (for (_ _array_index) _returnvalue
        (`PrimitiveComponent.SetMaterial` _ghostbuilding_mesh _array_index "/Game/MyRTSGame/Materials/GhostErrorMaterial_Instance.GhostErrorMaterial_Instance"))
      (else
        (for (_ _array_index_2) _returnvalue
          (`PrimitiveComponent.SetMaterial` _ghostbuilding_mesh _array_index_2 "/Game/MyRTSGame/Materials/GhostMaterial_Instance.GhostMaterial_Instance"))))))

(fn `CheckOverlap`
  (returns (Overlapping :type Boolean))
  (return (> (`KismetArrayLibrary.Array_Length` (`self.GetOverlappingActors` "/Script/Engine.StaticMesh")) 0)))

(fn `GetConstructionStruct`
  (returns (ConstructionStruct :type "/Game/MyRTSGame/Structs/Construction_Struct Structure"))
  (return (make `/Game/MyRTSGame/Structs/Construction_Struct` (`self.BuildingClass`) (`self.ConstructionProxy`) (`KismetMathLibrary.MakeTransform` (`self.K2_GetActorLocation`) (`self.K2_GetActorRotation`)) (`self.DisplayMesh`) 0.0)))

(fn `SetCursorPosition`
  (params (CursorLocation :type "Vector Structure"))
  (set `self.CursorWorldPosition` CursorLocation)
  (return))

(fn `SetGridSnapVector`
  (returns (GridSnap :type "Vector Structure"))
  (bind (_cursorworldposition_x _cursorworldposition_y _cursorworldposition_z) (`KismetMathLibrary.BreakVector` (`self.CursorWorldPosition`)))
  (bind _gridsize (`self.GridSize`))
  (return (`KismetMathLibrary.MakeVector` (`/Game/MyRTSGame/Libraries/FunctionLibrary.GridSnap` _cursorworldposition_x _gridsize) (`/Game/MyRTSGame/Libraries/FunctionLibrary.GridSnap` _cursorworldposition_y _gridsize) (`/Game/MyRTSGame/Libraries/FunctionLibrary.GridSnap` _cursorworldposition_z _gridsize))))

(fn `UserConstructionScript`)