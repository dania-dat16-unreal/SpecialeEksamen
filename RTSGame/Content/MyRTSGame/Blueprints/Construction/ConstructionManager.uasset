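; ConstructionManager is a Blueprint that manages building construction in an RTS, from queued request to finished structure.
; QueueConstruction spawns an actor from the construction struct's class and transform, ignoring collisions, then calls the completion-binding event.
; That event subscribes to a proxy's ConstructionCompleted notification.
; On completion, FinishConstruction spawns the configured building class at the configured transform and destroys the proxy.
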(event Custom|BindConstructionComplete
  (params (Proxy :type Construction%20Proxy%20Object%20Reference))
  (EventDispatchers|BindEventtoConstructionCompleted Proxy (EventDispatchers|CreateEvent :!event Custom|ConstructionCompleted)))

(event Custom|ConstructionCompleted
  (params (Proxy :type Construction%20Proxy%20Object%20Reference))
  (CallFunction|FinishConstruction Proxy))

(event EventBeginPlay)

(event EventActorBeginOverlap
  (params (OtherActor :type Actor%20Object%20Reference)))

(event EventTick
  (params (DeltaSeconds :type Float%20%28single-precision%29)))

(fn ConstructionScript)

(fn QueueConstruction
  (params (ConstructionStruct :type Construction%20Struct%20Structure))
  (bind (_buildingclass _proxyclass _transform) (Utilities|Struct|BreakConstruction_Struct ConstructionStruct))
  (Game|SpawnActorfromClass _buildingclass _transform "AlwaysSpawn" 0 0 0 0.0 0.0)
  (CallFunction|BindConstructionComplete))

(fn FinishConstruction
  (params (Proxy :type Construction%20Proxy%20Object%20Reference))
  (bind _config (LocalVariables|GetConfig))
  (bind (_buildingclass _proxyclass _transform) (Utilities|Struct|BreakConstruction_Struct _config))
  (Game|SpawnActorfromClass _buildingclass _transform "Undefined" 0 0 0 0.0 0.0)
  (Actor|DestroyActor Proxy))