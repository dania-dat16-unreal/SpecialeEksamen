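; Factory building Blueprint for an RTS, which starts below its placed position for construction.
; On BeginPlay it sets its name, stores its location as the build lerp position, then drops itself 2000 units.
; Tick passes delta time to a Build function, defined outside these graphs, while IsBuilding is true.
; The construction script only calls the parent's.
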(event `self.ReceiveBeginPlay`
  (bind _returnvalue (`self.K2_GetActorLocation`))
  (set `self.BuildingName` "Factory")
  (set `self.BuildLerpPosition` _returnvalue)
  (`self.K2_SetActorLocation` (- _returnvalue (0.0 0.0 2000.0))))

(event `self.ReceiveTick`
  (params (DeltaSeconds :type "Float (single-precision)"))
  (if (`self.IsBuilding`)
    (`self.Build` DeltaSeconds)))

(fn `UserConstructionScript`
  (`parent.UserConstructionScript`))