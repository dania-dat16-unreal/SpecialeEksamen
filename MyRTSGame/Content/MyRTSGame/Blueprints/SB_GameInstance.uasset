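; SB_GameInstance is a Game Instance Blueprint that handles multiplayer session joining, leaving and connection errors.
; JoinToSelectedServer joins the given search result for the first player controller, or prints a server-full message when no slots remain.
; DisconnectFromServer destroys that player's session.
; Network errors print the failure type and server flag, then destroy the session, while travel errors only print the failure type.
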(event `JoinToSelectedServer`
  (params (SearchResult :type "BlueprintSessionResult Structure (by ref)"))
  ;[1 1 1] Join a specific Server
  (if (< (`FindSessionsCallbackProxy.GetCurrentPlayers` SearchResult) (`FindSessionsCallbackProxy.GetMaxPlayers` SearchResult))
    ;;[1 1 1] Joinable Server
    (`JoinSessionCallbackProxy.JoinSession` (`GameplayStatics.GetPlayerController` 0) SearchResult)
    (else
      (`KismetSystemLibrary.PrintString` "Server Full" true true (struct :`G` 0.66 :`B` 1.0 :`A` 1.0) 10.0))))

(event `DisconnectFromServer`
  ;[1 1 1] Disconnect from server
  (`DestroySessionCallbackProxy.DestroySession` (`GameplayStatics.GetPlayerController` 0)))

(event `self.HandleNetworkError`
  (params (FailureType :type "ENetworkFailure Enum" :default "NetDriverAlreadyExists") (bIsServer :type Boolean))
  ;[1 1 1] If Network error (Someone has lost connection etc.) - Cleanup session
  (`KismetSystemLibrary.PrintString` (`KismetStringLibrary.Concat_StrStr` "Type: " (`|GetEnumeratorNameAsString` FailureType) "Server: " (`KismetStringLibrary.Conv_BoolToString` bIsServer) ">NETWORK ERROR") true true (struct :`G` 0.66 :`B` 1.0 :`A` 1.0) 10.0)
  (`DestroySessionCallbackProxy.DestroySession` (`GameplayStatics.GetPlayerController` 0)))

(event `self.HandleTravelError`
  (params (FailureType :type "ETravelFailure Enum" :default "NoLevel"))
  ;[1 1 1] What to do if travel to new level has error
  (`KismetSystemLibrary.PrintString` (`KismetStringLibrary.Concat_StrStr` "Type: " (`|GetEnumeratorNameAsString` FailureType) "Travel Error")))