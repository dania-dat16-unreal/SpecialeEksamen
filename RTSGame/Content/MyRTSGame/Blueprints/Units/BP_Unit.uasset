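; BP_Unit is an RTS unit that can be selected, ordered to move, and automatically shoots nearby targets.
; A range sphere sized to AttackRange collects other units and buildings without a team check.
; MasterTick prunes dead units, updates the material health parameter, runs AIMoveTo toward requested goals, and faces the closest target, spawning bullets on a cooldown.
; Damage lowers UnitMasterScript health, and selection toggles a material parameter.
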(event `Master Tick`
  (params (DeltaTime :type "Float (double-precision)"))
  (bind _unitmasterscript (`self.UnitMasterScript`))
  ;[1 1 1] Update text and move unit
  (`|ExecutionSequence`
    (:`then_0`
      (for (_array_element _array_index) (`self.EnemiesInRange`)
        (bind _asbp_unit (cast `/Game/MyRTSGame/Blueprints/Units/BP_Unit` _array_element)
          (:`then`
            (if (<= (`UnitMasterScript.CurrentHealth` (`/Game/MyRTSGame/Blueprints/Units/BP_Unit.UnitMasterScript` _asbp_unit)) 0.0)
              (`KismetArrayLibrary.Array_Remove` (`self.EnemiesInRange`) _array_index)))
          (:`CastFailed`
            (bind _asbuilding_master (cast `/Game/MyRTSGame/Blueprints/Buildings/BuildingMaster` _array_element))
            (if (<= 10.0 0.0)
              (`KismetArrayLibrary.Array_Remove` (`self.EnemiesInRange`) _array_index))))))
    (:`then_1`
      (if (<= (`UnitMasterScript.CurrentHealth` (`self.UnitMasterScript`)) 0.0)
        (set `self.bAutoDestroyWhenFinished` true)))
    (:`then_2`
      (`MaterialInstanceDynamic.SetScalarParameterValue` (`self.Material`) "MatHealthParam" (/ (mod (`UnitMasterScript.CurrentHealth` _unitmasterscript) (+ (`UnitMasterScript.MaxHealth` _unitmasterscript) 1.0)) 100.0))
      (if (`self.HasNewGoal`)
        (bind _returnvalue (`AIBlueprintHelperLibrary.GetAIController` self))
        (`KismetSystemLibrary.PrintString` (`KismetSystemLibrary.GetDisplayName` _returnvalue))
        (`AITask_MoveTo.AIMoveTo` _returnvalue (`self.Goal`)
          (:`OnMoveFinished`
            (set `self.HasNewGoal` false)))))
    (:`then_3`
      (if (>= (`KismetArrayLibrary.Array_Length` (`self.EnemiesInRange`)) 1)
        (bind _output_get (set `self.ClosestDistance` 10000.0))
        (for _array_element_2 (`self.EnemiesInRange`)
          (bind _returnvalue_2 (`self.GetDistanceTo` _array_element_2))
          (if (< _returnvalue_2 _output_get)
            (set `self.ClosestDistance` _returnvalue_2)
            (set `self.EnemyToFight` _array_element_2)))
        (`self.LookAtEnemy`)
        (if (< (`self.GetDistanceTo` (`self.EnemyToFight`) self) (`self.AttackRange`))
          (`self.FireWeapon`))
        (else
          (set `self.IsFighting2` false)
          (set `self.EnemyToFight` null))))
    (:`then_4`
      (set `self.ShootCooldown` (- (`self.ShootCooldown`) DeltaTime)))))

(event `self.Range.OnComponentBeginOverlap`
  (params (OtherActor :type "Actor Object Reference") (OtherComp :type "PrimitiveComponent Object Reference") (OtherBodyIndex :type Integer) (bFromSweep :type Boolean) (SweepResult :type "HitResult Structure (by ref)"))
  (if (== OtherActor self)
    _
    (elif (not (`self.IsFighting2`))
      (cast `/Game/MyRTSGame/Blueprints/Units/BP_Unit` OtherActor
        (:`then`
          _)
        (:`CastFailed`
          (cast `/Game/MyRTSGame/Blueprints/Buildings/BuildingMaster` OtherActor)))
      (`KismetArrayLibrary.Array_Add` (`self.EnemiesInRange`) OtherActor))))

(event `self.ReceiveAnyDamage`
  (params (Damage :type "Float (single-precision)") (DamageType :type "DamageType Object Reference") (InstigatedBy :type "Controller Object Reference") (DamageCauser :type "Actor Object Reference"))
  (bind _unitmasterscript (`self.UnitMasterScript`))
  (set `UnitMasterScript.CurrentHealth` (- (`UnitMasterScript.CurrentHealth` _unitmasterscript) Damage) _unitmasterscript))

(event `self.Range.OnComponentEndOverlap`
  (params (OtherActor :type "Actor Object Reference") (OtherComp :type "PrimitiveComponent Object Reference") (OtherBodyIndex :type Integer))
  (`KismetArrayLibrary.Array_Remove` (`self.EnemiesInRange`) (`KismetArrayLibrary.Array_Find` (`self.EnemiesInRange`) OtherActor)))

(event `LookAtEnemy`
  ;[1 1 1] FaceEnemy
  (`self.SetActorRotation` (`KismetMathLibrary.FindLookAtRotation` (`self.K2_GetActorLocation`) (`self.K2_GetActorLocation` (`self.EnemyToFight`)))))

(event `self.ReceiveBeginPlay`
  (`SphereComponent.SetSphereRadius` (`self.Range`) (`self.AttackRange`) true))

(event `FireWeapon`
  (bind _returnvalue (`SceneComponent.K2_GetComponentLocation` (`self.BowEnd`)))
  ;[1 1 1] FireWeapon
  (if (<= (`self.ShootCooldown`) 0.0)
    (`|SpawnActorFromClass` "/Game/MyRTSGame/Blueprints/Bullet.Bullet_C" (`KismetMathLibrary.MakeTransform` _returnvalue (`KismetMathLibrary.FindLookAtRotation` _returnvalue (`self.K2_GetActorLocation` (`self.EnemyToFight`))) (1.0 1.0 1.0)) "Undefined" "OverrideRootScale" null self)
    (set `self.ShootCooldown` 1.0)))

(fn `DeSelect`
  ;[1 1 1] Delet Text When Deselected
  (`MaterialInstanceDynamic.SetScalarParameterValue` (`self.Material`) "SelectedAmount" 0.0))

(fn `MoveRequest`
  (params (GoalLocation :type "Vector Structure"))
  ;[1 1 1] Sets has new Goal to True
  (set `self.Goal` GoalLocation)
  (set `self.HasNewGoal` true))

(fn `Select`
  (params (OwningPlayer :type "/Game/MyRTSGame/Blueprints/CameraPawn Object Reference"))
  ;[1 1 1] Set Text When Selected
  (`MaterialInstanceDynamic.SetScalarParameterValue` (`self.Material`) "SelectedAmount" 1000.0))

(fn `UserConstructionScript`)