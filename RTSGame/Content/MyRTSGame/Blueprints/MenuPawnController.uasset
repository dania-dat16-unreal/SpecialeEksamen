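; Menu controller Blueprint that exposes screen settings (resolution, fullscreen and VSync) for the game's menu.
; It is a thin wrapper around MenuCPP, which does the actual work in what appears to be C++.
; The ApplyScreenSettings event forwards values to MenuCPP, while GetScreenSettings refreshes MenuCPP and returns its stored values.
; BeginPlay, Tick and the construction script are empty.
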(event `ApplyScreenSettings`
  (params (Resolution :type String) (Fullscreen :type Boolean) (`V-Sync` :type Boolean))
  (`MenuCPP.ApplyScreenSettings` (`self.MenuCPP`) Resolution Fullscreen `V-Sync`))

(fn `GetScreenSettings`
  (returns (Resolution :type String) (Fullscreen :type Boolean) (Vsync :type Boolean))
  (bind _menucpp (`self.MenuCPP`))
  (`MenuCPP.GetScreenSettings` _menucpp)
  (return (`MenuCPP.resolutionOptionCPP` _menucpp) (`MenuCPP.fullscreenCPP` _menucpp) (`MenuCPP.vsyncCPP` _menucpp)))

(fn `UserConstructionScript`)