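; BP_Soldier is the soldier unit Blueprint for an RTS game.
; Its construction script creates a dynamic material from BP_SoldierMat on the mesh, zeroes the health and selection parameters, and sets the unit's production time.
; Tick calls MasterTick with a zero argument rather than delta time, then re-assigns a take-any-damage handler every frame, though that handler is empty.
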(event `self.ReceiveTick`
  (params (DeltaSeconds :type "Float (single-precision)"))
  (`|ExecutionSequence`
    (:`then_0`
      (`self.Master Tick` 0.0))
    (:`then_1`
      (add `self.OnTakeAnyDamage` (delegate `OnTakeAnyDamage_Event_0`)))))

(event `OnTakeAnyDamage_Event_0` :!signature `self.OnTakeAnyDamage`
  (params (Damage :type "Float (double-precision)") (DamageType :type "DamageType Object Reference") (InstigatedBy :type "Controller Object Reference") (DamageCauser :type "Actor Object Reference")))

(fn `UserConstructionScript`
  (bind _returnvalue (`PrimitiveComponent.CreateDynamicMaterialInstance` (`self.Mesh`) 0 "/Game/MyRTSGame/Blueprints/Units/Soldier/BP_SoldierMat.BP_SoldierMat"))
  (`MaterialInstanceDynamic.SetScalarParameterValue` _returnvalue "MatHealthParam" 0.0)
  (`MaterialInstanceDynamic.SetScalarParameterValue` _returnvalue "SelectedAmount" 0.0)
  (set `self.Material` _returnvalue)
  (set `self.ProductionTime` 5.0))