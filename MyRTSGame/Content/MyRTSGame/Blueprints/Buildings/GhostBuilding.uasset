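; Ghost building actor that previews building placement in the RTS build mode.
; While active, a gated Tick snaps it to the grid at the externally set cursor position and swaps to an error material on overlap.
; ConstructBuilding briefly spawns the building to read its proxy and display mesh, restarts the ghost with them, then destroys that instance.
; GetConstructionStruct packages the class, proxy, mesh and ghost transform for construction.
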(event `OnSpawn`
  (params (BuildingClass :type "/Game/MyRTSGame/Blueprints/Buildings/BuildingMaster Class Reference") (ConstructionProxy :type "/Game/MyRTSGame/Blueprints/Construction/ConstructionProxy Class Reference") (DisplayMesh :type "StaticMesh Object Reference"))
  ;[1 1 1] On spawn ghost
  (if (not (`self.IsActive`))
    (set `self.BuildingClass` BuildingClass)
    (set `self.ConstructionProxy` ConstructionProxy)
    (set `self.DisplayMesh` DisplayMesh)
    (set `self.IsActive` true)
    (set `/Game/MyRTSGame/Blueprints/CameraPawnController.BuildModeActive` true (`self.ControllerRef`))
    (`StaticMeshComponent.SetStaticMesh` (`self.GhostBuilding_Mesh`) (`self.DisplayMesh`))
    (`self.OpenTickGate`)
    (`self.SetMaterial` (not (`self.IsOverlapping`)))))

(event `KillGhost`
  ;[1 1 1] Kill ghost
  (set `self.BuildingClass` null)
  (set `self.ConstructionProxy` null)
  (`self.CloseTickGate`)
  (set `self.DisplayMesh` null)
  (set `self.IsActive` false)
  (set `/Game/MyRTSGame/Blueprints/CameraPawnController.BuildModeActive` false (`self.ControllerRef`))
  (`StaticMeshComponent.SetStaticMesh` (`self.GhostBuilding_Mesh`) (`self.DisplayMesh`)))

(event `/Game/MyRTSGame/Interfaces/I_HUD.ConstructBuilding`
  (params (MainBuilding :type "/Game/MyRTSGame/Blueprints/Buildings/BuildingMaster Class Reference"))
  ;[1 1 1] Construct building
  (bind _returnvalue (`|SpawnActorFromClass` MainBuilding (`KismetMathLibrary.MakeTransform` (0.0 0.0 0.0)) "Undefined" "OverrideRootScale" null (`self.ControllerRef`)))
  (`|ExecutionSequence`
    (:`then_0`
      (bind _asbuilding_master (castclass `/Game/MyRTSGame/Blueprints/Buildings/BuildingMaster` MainBuilding))
      (`self.KillGhost`)
      (`self.OnSpawn` _asbuilding_master (`/Game/MyRTSGame/Blueprints/Buildings/BuildingMaster.ConstructionProxy` _returnvalue) (`/Game/MyRTSGame/Blueprints/Buildings/BuildingMaster.DisplayMesh` _returnvalue)))
    (:`then_1`
      (`self.K2_DestroyActor` _returnvalue))))

(event `self.ReceiveTick`
  (params (DeltaSeconds :type "Float (single-precision)"))
  ;[1 1 1] Tick
  (`/Engine/EditorBlueprintResources/StandardMacros.Gate` true :!label _label
    (:`Exit`
      (`self.K2_SetActorLocation` self (`self.SetGridSnapVector`) false false)
      (if (`self.CheckOverlap`)
        (`self.SetMaterial` true)
        (else
          (`self.SetMaterial` false))))))

(event `OpenTickGate`
  ;[1 1 1] Tick
  (goto _label :!via `Open`))

(event `CloseTickGate`
  ;[1 1 1] Tick
  (goto _label :!via `Close`))

(event `SetMaterial`
  (params (IsError :type Boolean))
  (bind _ghostbuilding_mesh (`self.GhostBuilding_Mesh`))
  ;[1 1 1] Set material on building depending on overlap
  (if (not (== IsError (`self.IsOverlapping`)))
    (bind _output_get (set `self.IsOverlapping` IsError))
    (if _output_get
      (`PrimitiveComponent.SetMaterial` _ghostbuilding_mesh 0 "/Game/MyRTSGame/Materials/GhostErrorMaterial_Instance.GhostErrorMaterial_Instance")
      (else
        (`PrimitiveComponent.SetMaterial` _ghostbuilding_mesh 0 "/Game/MyRTSGame/Materials/GhostMaterial_Instance.GhostMaterial_Instance")))))

(fn `CheckOverlap`
  (returns (Overlapping :type Boolean))
  (return (> (`KismetArrayLibrary.Array_Length` (`self.GetOverlappingActors` "/Script/Engine.Actor")) 0)))

(fn `GetConstructionStruct`
  (returns (ConstructionStruct :type "/Game/MyRTSGame/Structs/Construction_Struct Structure"))
  (return (make `/Game/MyRTSGame/Structs/Construction_Struct` (`self.BuildingClass`) (`self.ConstructionProxy`) (`KismetMathLibrary.MakeTransform` (`self.K2_GetActorLocation`) (`self.K2_GetActorRotation`)) (`self.DisplayMesh`) 0.0)))

(fn `SetCursorPosition`
  (params (CursorLocation :type "Vector Structure"))
  (set `self.CursorWorldPosition` CursorLocation)
  (return))

(fn `SetGridSnapVector`
  (returns (GridSnap :type "Vector Structure"))
  (bind (_cursorworldposition_x _cursorworldposition_y _cursorworldposition_z) (`KismetMathLibrary.BreakVector` (`self.CursorWorldPosition`)))
  (bind _gridsize (`self.GridSize`))
  (return (`KismetMathLibrary.MakeVector` (`/Game/MyRTSGame/Libraries/FunctionLibrary.GridSnap` _cursorworldposition_x _gridsize) (`/Game/MyRTSGame/Libraries/FunctionLibrary.GridSnap` _cursorworldposition_y _gridsize) (`/Game/MyRTSGame/Libraries/FunctionLibrary.GridSnap` _cursorworldposition_z _gridsize))))

(fn `UserConstructionScript`)