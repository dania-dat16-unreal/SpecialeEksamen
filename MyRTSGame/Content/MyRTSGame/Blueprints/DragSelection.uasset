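; DragSelection is an RTS HUD that draws a drag rectangle and gathers the units under it.
; While IsDrawing is true, DrawHUD stretches a texture from ClickedLocation to the mouse each frame.
; It deprojects the rectangle's center and box-traces WorldDynamic objects along that ray, using raw pixel extents, axes swapped, as world-space half-size.
; Hit BP_Unit actors are added uniquely to SelectedActor and never removed here.
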(event `self.ReceiveDrawHUD`
  (params (SizeX :type Integer) (SizeY :type Integer))
  (bind _returnvalue (`GameplayStatics.GetPlayerController` 0))
  (bind (_locationx _locationy) (`PlayerController.GetMousePosition` _returnvalue))
  (bind (_x _y) (`KismetMathLibrary.BreakVector2D` (`self.ClickedLocation`)))
  (bind (_x_2 _y_2) (`KismetMathLibrary.BreakVector2D` (- (`self.MouseLocation`) (`self.ClickedLocation`))))
  (bind (_x_3 _y_3) (`KismetMathLibrary.BreakVector2D` (- (`self.MouseLocation`) (`self.ClickedLocation`))))
  (bind (_x_4 _y_4) (`KismetMathLibrary.BreakVector2D` (/ (+ (`self.ClickedLocation`) (`self.MouseLocation`)) 2.0)))
  (bind (_worldlocation _worlddirection) (`PlayerController.DeprojectScreenPositionToWorld` _returnvalue _x_4 _y_4))
  ;[1 1 1] DragToSelect
  (set `self.ScreenReselution` (`KismetMathLibrary.MakeVector2D` (`KismetMathLibrary.Conv_IntToDouble` SizeX) (`KismetMathLibrary.Conv_IntToDouble` SizeY)))
  (if (`self.IsDrawing`)
    (set `self.MouseLocation` (`KismetMathLibrary.MakeVector2D` _locationx _locationy))
    (`self.DrawTexture` "/Game/StarterContent/Textures/T_Brick_Clay_Beveled_D.T_Brick_Clay_Beveled_D" _x _y _x_3 _y_3)
    (bind _outhits (`KismetSystemLibrary.BoxTraceMultiForObjects` _worldlocation (+ _worldlocation (* _worlddirection 10000.0)) (`KismetMathLibrary.MakeVector` (`KismetMathLibrary.Abs` _y_2) (`KismetMathLibrary.Abs` _x_2) 20.0) (struct) (`|MakeArray` "ObjectTypeQuery2" :!type "EObjectTypeQuery Enum")))
    (for _array_element _outhits
      (bind (_bblockinghit _binitialoverlap _time _location _impactpoint _normal _impactnormal _physmat _hitactor) (`GameplayStatics.BreakHitResult` _array_element))
      (cast `/Game/MyRTSGame/Blueprints/BP_Unit` _hitactor)
      (if (not (`KismetArrayLibrary.Array_Contains` (`self.SelectedActor`) _hitactor))
        (`KismetArrayLibrary.Array_Add` (`self.SelectedActor`) _hitactor)))))

(fn `UserConstructionScript`)