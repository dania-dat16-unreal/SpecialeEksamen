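; Projectile actor for the RTS game that damages units and buildings it overlaps.
; On spawn, its Bullet component ignores the FiredFrom actor when moving, and the actor destroys itself after a fixed lifetime.
; Overlapping any actor other than the shooter destroys it, first applying fixed damage credited to FiredFrom if the target is a BP_Unit or BuildingMaster.
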(event `self.ReceiveBeginPlay`
  (`PrimitiveComponent.IgnoreActorWhenMoving` (`self.Bullet`) (`self.FiredFrom`) true)
  (`KismetSystemLibrary.Delay` 10.0)
  (`self.K2_DestroyActor`))

(event `self.ReceiveActorBeginOverlap`
  (params (OtherActor :type "Actor Object Reference"))
  (bind _firedfrom (`self.FiredFrom`))
  (if (not (== OtherActor _firedfrom))
    (cast `/Game/MyRTSGame/Blueprints/Units/BP_Unit` OtherActor
      (:`then`
        (`GameplayStatics.ApplyDamage` OtherActor 10.0 null _firedfrom :!label _label))
      (:`CastFailed`
        (cast `/Game/MyRTSGame/Blueprints/Buildings/BuildingMaster` OtherActor
          (:`then`
            (goto _label))
          (:`CastFailed`
            _))))
    (`self.K2_DestroyActor`)))

(fn `UserConstructionScript`)