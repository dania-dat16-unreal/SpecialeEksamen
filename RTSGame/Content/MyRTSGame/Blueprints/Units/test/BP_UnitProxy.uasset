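; BP_UnitProxy is an actor that stands in for an RTS unit and follows it around.
; On BeginPlay, the authority spawns a BP_Unit2 and a BP_UnitAI controller at the proxy's transform, then has the controller possess the unit.
; Unit and AIcontroller have empty RepNotify handlers.
; Each tick, the proxy moves halfway toward the unit's transform, giving frame-rate-dependent smoothing wherever the Unit reference is valid.
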(event `self.ReceiveBeginPlay`
  (bind _returnvalue (`self.GetTransform`))
  (`/Engine/EditorBlueprintResources/ActorMacros.Switch Has Authority`
    (:`Authority`
      (bind _returnvalue_2 (`|SpawnActorFromClass` "/Game/MyRTSGame/Blueprints/Units/test/BP_Unit2.BP_Unit2_C" _returnvalue "Undefined" "OverrideRootScale"))
      (set `self.Unit` _returnvalue_2)
      (bind _returnvalue_3 (`|SpawnActorFromClass` "/Game/MyRTSGame/Blueprints/Units/test/BP_UNITAI.BP_UnitAI_C" _returnvalue "Undefined" "OverrideRootScale"))
      (bind _output_get (set `self.AIcontroller` _returnvalue_3))
      (`Controller.Possess` _output_get (`self.Unit`)))))

(event `self.ReceiveTick`
  (params (DeltaSeconds :type "Float (single-precision)"))
  (bind _unit (`self.Unit`))
  (`/Engine/EditorBlueprintResources/StandardMacros.IsValid` _unit
    (:`Is Valid`
      (`self.K2_SetActorTransform` (`KismetMathLibrary.TLerp` (`self.GetTransform` _unit) (`self.GetTransform`) 0.5)))))

(fn `OnRep_AIcontroller`)

(fn `OnRep_Unit`)

(fn `UserConstructionScript`)