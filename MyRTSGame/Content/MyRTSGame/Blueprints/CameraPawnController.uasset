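; RTS camera controller that drives the CameraPawn with keyboard movement, screen-edge scrolling, mouse panning and zoom.
; Key movement follows the pawn's facing, with speed scaled by spring-arm length and boosted by Left Shift, which also speeds edge scrolling.
; Holding Pan opens gates that turn mouse motion into yaw and clamped pitch while disabling navigation; PanReset levels pitch.
; Zoom inputs step the spring-arm length within clamped limits.
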(event `self.ReceiveBeginPlay`
  ;[1 1 1] Get camera pawn reference
  (`|ExecutionSequence`
    (:`then_0`
      (`self.ReferenceCasts`))))

(event `InputAxis|MoveForward`
  (params (AxisValue :type "Float (single-precision)"))
  ;[1 1 1] Keyboard movement X
  (if (not (`self.DisableCamNav`))
    (`self.K2_SetActorTransform` (`self.CameraPawnRef`) (`self.MovementX` (`self.MovementSpeedCalculation`) (`self.FastMoveMultiplier`) AxisValue (`self.CameraPawnRef`)) false false)))

(event `InputAxisKey|MouseX`
  (params (AxisValue :type "Float (single-precision)"))
  ;[1 1 1] Mouse edge movement
  (if (not (`self.DisableCamNav`))
    (bind (_deltaxspeed _deltayspeed) (`self.ScreenEdgeMovement` :!label _label))
    (`self.K2_AddActorLocalOffset` (`self.CameraPawnRef`) (`KismetMathLibrary.MakeVector` _deltaxspeed _deltayspeed) true false)))

(event `InputAxisKey|MouseY`
  (params (AxisValue :type "Float (single-precision)"))
  ;[1 1 1] Mouse edge movement
  (if (not (`self.DisableCamNav`))
    (goto _label :!via `MouseY`)))

(event `InputAxis|MoveRight`
  (params (AxisValue :type "Float (single-precision)"))
  ;[1 1 1] Keyboard movement Y
  (if (not (`self.DisableCamNav`))
    (`self.K2_SetActorTransform` (`self.CameraPawnRef`) (`KismetMathLibrary.MakeTransform` (`KismetMathLibrary.MakeVector` (.x (.location (`self.MovementY` AxisValue (`self.MovementSpeedCalculation`) (`self.FastMoveMultiplier`) (`self.CameraPawnRef`)))) (.y (.location (`self.MovementY` AxisValue (`self.MovementSpeedCalculation`) (`self.FastMoveMultiplier`) (`self.CameraPawnRef`)))) 100.0) (.rotation (`self.MovementY` AxisValue (`self.MovementSpeedCalculation`) (`self.FastMoveMultiplier`) (`self.CameraPawnRef`))) (.scale (`self.MovementY` AxisValue (`self.MovementSpeedCalculation`) (`self.FastMoveMultiplier`) (`self.CameraPawnRef`)))) false false)))

(event `Key|LeftShift`
  (params (Key :type "Key Structure" :default "AnyKey"))
  ;[1 1 1] Movement speed
  (:`Pressed`
    (set `self.FastMoveMultiplier` 2.0))
  (:`Released`
    (set `self.FastMoveMultiplier` 1.0)))

(event `InputAxisKey|MouseX`
  (params (AxisValue :type "Float (single-precision)"))
  ;[1 1 1] Pan X axis
  (`/Engine/EditorBlueprintResources/StandardMacros.Gate` true :!label _label_2
    (:`Exit`
      (`self.SetActorRotation` (`self.CameraPawnRef`) (`KismetMathLibrary.MakeRotator` (.roll (`self.K2_GetActorRotation` (`self.CameraPawnRef`))) (.pitch (`self.K2_GetActorRotation` (`self.CameraPawnRef`))) (+ (.yaw (`self.K2_GetActorRotation` (`self.CameraPawnRef`))) (* (`self.PanSensitivity`) AxisValue)))))))

(event `InputAction|PanReset`
  (params (Key :type "Key Structure" :default "AnyKey"))
  (bind _camerapawnref (`self.CameraPawnRef`))
  ;[1 1 1] Pan reset
  (:`Pressed`
    (`self.SetActorRotation` _camerapawnref (`KismetMathLibrary.MakeRotator` (.roll (`self.K2_GetActorRotation` _camerapawnref)) 0.0 (.yaw (`self.K2_GetActorRotation` _camerapawnref))))))

(event `InputAction|Pan`
  (params (Key :type "Key Structure" :default "AnyKey"))
  ;[1 1 1] Pan X axis
  (:`Pressed`
    (set `self.DisableCamNav` true)
    (goto _label_2 :!via `Open`))
  (:`Released`
    (set `self.DisableCamNav` false)
    (goto _label_2 :!via `Close`)))

(event `InputAxisKey|MouseY`
  (params (AxisValue :type "Float (single-precision)"))
  ;[1 1 1] Pan Y axis
  (`/Engine/EditorBlueprintResources/StandardMacros.Gate` true :!label _label_3
    (:`Exit`
      (`self.SetActorRotation` (`self.CameraPawnRef`) (`KismetMathLibrary.MakeRotator` (.roll (`self.K2_GetActorRotation` (`self.CameraPawnRef`))) (`KismetMathLibrary.FClamp` (+ (.pitch (`self.K2_GetActorRotation` (`self.CameraPawnRef`))) (* (`self.PanSensitivity`) AxisValue)) -15.0 45.0) (.yaw (`self.K2_GetActorRotation` (`self.CameraPawnRef`))))))))

(event `InputAction|Pan`
  (params (Key :type "Key Structure" :default "AnyKey"))
  ;[1 1 1] Pan Y axis
  (:`Pressed`
    (set `self.DisableCamNav` true)
    (goto _label_3 :!via `Open`))
  (:`Released`
    (set `self.DisableCamNav` false)
    (goto _label_3 :!via `Close`)))

(event `InputAction|ZoomIn`
  (params (Key :type "Key Structure" :default "AnyKey"))
  (bind _springarm (`/Game/MyRTSGame/Blueprints/CameraPawn.SpringArm` (`self.CameraPawnRef`)))
  ;[1 1 1] Zoom in/out
  (:`Pressed`
    (set `SpringArmComponent.TargetArmLength` (`KismetMathLibrary.FClamp` (- (`SpringArmComponent.TargetArmLength` _springarm) (`self.ZoomSensitivity`)) 500.0 (`self.MaxArmDistance`)) _springarm)))

(event `InputAction|ZoomOut`
  (params (Key :type "Key Structure" :default "AnyKey"))
  (bind _springarm (`/Game/MyRTSGame/Blueprints/CameraPawn.SpringArm` (`self.CameraPawnRef`)))
  ;[1 1 1] Zoom in/out
  (:`Pressed`
    (set `SpringArmComponent.TargetArmLength` (`KismetMathLibrary.FClamp` (+ (`self.ZoomSensitivity`) (`SpringArmComponent.TargetArmLength` _springarm)) 500.0 (`self.MaxArmDistance`)) _springarm)))

(fn `MovementSpeedCalculation`
  (returns (MoveSensitivity :type "Float (double-precision)"))
  (return (`KismetMathLibrary.FClamp` (/ (`SpringArmComponent.TargetArmLength` (`/Game/MyRTSGame/Blueprints/CameraPawn.SpringArm` (`self.CameraPawnRef`))) 100.0) 5.0 20.0)))

(fn `UserConstructionScript`)