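; BP_Unit is an RTS unit that can be selected, shows its health through its material and moves to requested locations.
; Construction creates a dynamic material on the Cone, whose scalar parameters show selection via Select/DeSelect and health, refreshed every Tick.
; MoveRequest stores a goal and sets a flag; while it is set, Tick reissues AIMoveTo every frame until Move Finished clears it.
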(event `self.ReceiveTick`
  (params (DeltaSeconds :type "Float (single-precision)"))
  ;[1 1 1] Update text and move unit
  (`MaterialInstanceDynamic.SetScalarParameterValue` (`self.Material`) "MatHealthParam" (/ (mod (`self.CurrentHealth`) (+ (`self.MaxHealth`) 1.0)) 100.0))
  (if (`self.HasNewGoal`)
    (bind _returnvalue (`AIBlueprintHelperLibrary.GetAIController` self))
    (`AITask_MoveTo.AIMoveTo` _returnvalue (`self.Goal`)
      (:`OnMoveFinished`
        (set `self.HasNewGoal` false)))))

(fn `DeSelect`
  ;[1 1 1] Delet Text When Deselected
  (`MaterialInstanceDynamic.SetScalarParameterValue` (`self.Material`) "SelectedAmount" 0.0))

(fn `MoveRequest`
  (params (GoalLocation :type "Vector Structure"))
  ;[1 1 1] Sets has new Goal to True
  (set `self.Goal` GoalLocation)
  (set `self.HasNewGoal` true))

(fn `Select`
  (params (OwningPlayer :type "/Game/MyRTSGame/Blueprints/CameraPawn Object Reference"))
  ;[1 1 1] Set Text When Selected
  (`MaterialInstanceDynamic.SetScalarParameterValue` (`self.Material`) "SelectedAmount" 1000.0))

(fn `UserConstructionScript`
  (bind _returnvalue (`PrimitiveComponent.CreateDynamicMaterialInstance` (`self.Cone`) 0 "/Game/MyRTSGame/Blueprints/BP_UnitMat.BP_UnitMat"))
  (`MaterialInstanceDynamic.SetScalarParameterValue` _returnvalue "MatHealthParam" 0.0)
  (`MaterialInstanceDynamic.SetScalarParameterValue` _returnvalue "SelectedAmount" 0.0)
  (set `self.Material` _returnvalue)
  (set `self.ProductionTime` 5.0))