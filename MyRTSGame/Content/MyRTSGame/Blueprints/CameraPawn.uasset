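; CameraPawn is the RTS player pawn that selects units and orders them to move with mouse clicks.
; It caches its CameraPawnController on possession and uses it to trace from the cursor into the world on the Visibility channel.
; Releasing left click adds a hit BP_Unit to SelectedUnits, or deselects all otherwise.
; Releasing right click sends the hit location as a MoveRequest to every selected unit.
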(event `self.ReceivePossessed`
  (params (NewController :type "Controller Object Reference"))
  (bind _ascamera_pawn_controller (cast `/Game/MyRTSGame/Blueprints/CameraPawnController` NewController))
  (set `self.OwningController` _ascamera_pawn_controller))

(event `self.ReceiveUnpossessed`
  (params (OldController :type "Controller Object Reference"))
  (set `self.OwningController` null))

(event `Key|LeftMouseButton`
  (params (Key :type "Key Structure" :default "AnyKey"))
  (bind _selectedunits (`self.SelectedUnits`))
  ;[1 1 1] Select Units
  (:`Released`
    (bind _outhit (`self.LineTraceMouse`))
    (bind _asbp_unit (cast `/Game/MyRTSGame/Blueprints/BP_Unit` (`.HitActor` (`GameplayStatics.BreakHitResult` _outhit)))
      (:`then`
        (set `/Game/MyRTSGame/Blueprints/BP_Unit.IsSelected` true _asbp_unit)
        (`/Game/MyRTSGame/Blueprints/BP_Unit.Select` _asbp_unit self)
        (`KismetArrayLibrary.Array_Add` _selectedunits _asbp_unit))
      (:`CastFailed`
        (for _array_element _selectedunits
          (set `/Game/MyRTSGame/Blueprints/BP_Unit.IsSelected` false _array_element)
          (`/Game/MyRTSGame/Blueprints/BP_Unit.DeSelect` _array_element))
        (`KismetArrayLibrary.Array_Clear` _selectedunits)))))

(event `Key|RightMouseButton`
  (params (Key :type "Key Structure" :default "AnyKey"))
  ;[1 1 1] Move
  (:`Released`
    (bind (_outhit _hit) (`self.LineTraceMouse`))
    (if _hit
      (for _array_element (`self.SelectedUnits`)
        (`/Game/MyRTSGame/Blueprints/BP_Unit.MoveRequest` _array_element (`.Location` (`GameplayStatics.BreakHitResult` _outhit)))))))

(fn `LineTraceMouse`
  (returns (OutHit :type "HitResult Structure") (Hit :type Boolean))
  (bind _owningcontroller (`self.OwningController`))
  (bind (_worldlocation _worlddirection) (`PlayerController.DeprojectMousePositionToWorld` _owningcontroller))
  ;[1 1 1] Cast a line and detect hit
  (if (`KismetSystemLibrary.IsValid` _owningcontroller)
    (bind (_outhit _returnvalue) (`KismetSystemLibrary.LineTraceSingle` _worldlocation (+ _worldlocation (* _worlddirection 10000.0)) "TraceTypeQuery1"))
    (return _outhit _returnvalue)
    (else
      (return (struct) false))))

(fn `UserConstructionScript`)